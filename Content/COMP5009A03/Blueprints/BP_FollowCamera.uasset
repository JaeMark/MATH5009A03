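; Follow camera actor that tracks its parent component with X and Z offsets, intended for use as a child actor.
; Each Tick sets X directly from the parent, eases Z with FInterpTo for smoothed vertical follow, and keeps its current Y.
; ZoomInOut chains two timelines that lerp the X offset out to a zoomed-out value, then back to the default.
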(event `self.ReceiveBeginPlay`
  (set `self.CameraOffsetX` (`self.DefaultCameraOffsetX`)))

(event `self.ReceiveTick`
  (params (DeltaSeconds :type "Float (single-precision)"))
  (bind (_returnvalue_x _returnvalue_y) (`KismetMathLibrary.BreakVector` (`self.K2_GetActorLocation`)))
  (bind (_returnvalue_x_2 _returnvalue_y_2 _returnvalue_z) (`KismetMathLibrary.BreakVector` (`self.K2_GetActorLocation`)))
  (bind (_returnvalue_x_3 _returnvalue_y_3 _returnvalue_z_2) (`KismetMathLibrary.BreakVector` (+ (`SceneComponent.K2_GetComponentLocation` (`self.GetParentComponent`)) (`KismetMathLibrary.MakeVector` (`self.CameraOffsetX`) 0.0 (`self.CameraOffsetZ`)))))
  (`self.K2_SetActorLocation` (`KismetMathLibrary.MakeVector` _returnvalue_x_3 _returnvalue_y (`KismetMathLibrary.FInterpTo` _returnvalue_z _returnvalue_z_2 (`GameplayStatics.GetWorldDeltaSeconds`) 5.0))))

(event `ZoomInOut`
  (bind (_direction _newtrack_0) (`Timeline|ZoomOutTimeline` :!via `PlayFromStart`)
    (:`Update`
      (set `self.CameraOffsetX` (`KismetMathLibrary.Lerp` (`self.DefaultCameraOffsetX`) (`self.ZoomedOutCameraOffset`) _newtrack_0)))
    (:`Finished`
      (bind (_direction_2 _newtrack_0_2) (`Timeline|ZoomInTimeline` :!via `PlayFromStart`)
        (:`Update`
          (set `self.CameraOffsetX` (`KismetMathLibrary.Lerp` (`self.ZoomedOutCameraOffset`) (`self.DefaultCameraOffsetX`) _newtrack_0_2)))
        (:`Finished`
          (set `self.CameraOffsetX` (`self.DefaultCameraOffsetX`)))))))

(fn `UserConstructionScript`)