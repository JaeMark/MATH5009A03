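; Base actor for breakable static-mesh props that damage a pawn on contact and swap to a fracturable version.
; When a pawn begins overlapping the box, it takes fixed damage and the static mesh loses collision and is hidden.
; An actor of the configured geometry collection class then spawns at the mesh's world transform, with the pawn as instigator.
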(event `self.Box.OnComponentBeginOverlap`
  (params (OverlappedComponent :type "PrimitiveComponent Object Reference") (OtherActor :type "Actor Object Reference") (OtherComp :type "PrimitiveComponent Object Reference") (OtherBodyIndex :type Integer) (bFromSweep :type Boolean) (SweepResult :type "HitResult Structure (by ref)"))
  (bind _aspawn (cast `Pawn` OtherActor))
  (bind _output_get (set `self.HitPawn` _aspawn))
  (`GameplayStatics.ApplyDamage` _output_get 20.0)
  (`PrimitiveComponent.SetCollisionProfileName` (`self.StaticMesh`) "NoCollision" true)
  ;[0.276 0.276 0.276] Replace static mesh with fracturable mesh
  (`SceneComponent.SetHiddenInGame` (`self.StaticMesh`) true false)
  (`|SpawnActorFromClass` (`self.GeometryCollectionClass`) (`SceneComponent.K2_GetComponentToWorld` (`self.StaticMesh`)) "AlwaysSpawn" "MultiplyWithRoot" null (`self.HitPawn`)))

(fn `UserConstructionScript`)