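; Base fracturable mesh actor that breaks apart when something instigated by a player controller overlaps its box, damaging that overlapping actor.
; The overlap stores the impact normal, enables gravity on the Geometry Collection, then spawns and triggers an FS_MasterField at the impact point to drive the Chaos fracture.
; Chaos break events switch collision to the FractureCluster profile and apply a strong impulse along negative local up, nudged by the stored normal.
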(event `self.GeometryCollection.OnChaosBreakEvent`
  (params (BreakEvent :type "ChaosBreakEvent Structure (by ref)"))
  (bind _geometrycollection (`self.GeometryCollection`))
  (`PrimitiveComponent.SetCollisionProfileName` (`self.GeometryCollection`) "FractureCluster" true)
  (`PrimitiveComponent.AddImpulseAtLocation` _geometrycollection (+ (* (`SceneComponent.GetUpVector` _geometrycollection) -5000000.0) (* (`self.Sweep Result Impact Normal`) 10000.0)) BreakEvent_Location "None"))

(event `self.Box.OnComponentBeginOverlap`
  (params (OverlappedComponent :type "PrimitiveComponent Object Reference") (OtherActor :type "Actor Object Reference") (OtherComp :type "PrimitiveComponent Object Reference") (OtherBodyIndex :type Integer) (bFromSweep :type Boolean) (SweepResult :type "HitResult Structure (by ref)"))
  (set `self.Sweep Result Impact Normal` SweepResult_ImpactNormal)
  (if (`Controller.IsPlayerController` (`self.GetInstigatorController` OtherActor))
    (`GameplayStatics.ApplyDamage` OtherActor 20.0)
    (`PrimitiveComponent.SetEnableGravity` (`self.GeometryCollection`) true)
    (bind _returnvalue (`|SpawnActorFromClass` "/Engine/EditorResources/FieldNodes/FS_MasterField.FS_MasterField_C" (`KismetMathLibrary.MakeTransform` SweepResult_ImpactPoint) "Undefined" "MultiplyWithRoot" null null))
    (set `/Engine/EditorResources/FieldNodes/FS_MasterField.ActivationType` "NewEnumerator4" _returnvalue)
    (`/Engine/EditorResources/FieldNodes/FS_MasterField.CE_Trigger` _returnvalue)))

(fn `UserConstructionScript`)