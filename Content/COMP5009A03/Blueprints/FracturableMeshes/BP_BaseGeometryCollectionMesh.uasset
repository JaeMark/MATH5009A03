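; Base fracturable mesh actor that launches its Geometry Collection as soon as it spawns.
; On BeginPlay it applies an impulse at the actor location, summing the collection's up vector scaled by a vertical impulse and the instigator's forward vector scaled by a normal impulse.
; The debris therefore flies upward and along the direction the instigator faces.
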(event `self.ReceiveBeginPlay`
  (`PrimitiveComponent.AddImpulseAtLocation` (`self.GeometryCollection`) (+ (* (`SceneComponent.GetUpVector` (`self.GeometryCollection`)) (`self.VerticalImpulse`)) (* (`self.GetActorForwardVector` (`self.GetInstigator`)) (`self.NormalImpulse`))) (`self.K2_GetActorLocation`) "None"))

(fn `UserConstructionScript`)